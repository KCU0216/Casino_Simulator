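; Drunk NPC enemy character with modular clothing, ambient idle sounds and a hit reaction hook.
; On BeginPlay the shirt, trousers and boots meshes follow the main Mesh through leader pose.
; A self-rescheduling timer plays the drunk idle SFX at the actor's location through CasinoSoundSubsystem, at random intervals of a few seconds.
; RequestHitReaction forwards the attacker to HandleEnemyHitReaction.
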(event `ScheduleNextDrunkSound`
  (`KismetSystemLibrary.K2_SetTimerDelegate` (delegate `PlayDrunkSound`) (`KismetMathLibrary.RandomFloatInRange` 3.0 10.0)))

(event `PlayDrunkSound`
  (`CasinoSoundSubsystem.PlaySFX` (subsystem `CasinoSoundSubsystem`) "NPC_Drunk_Idle" true (`self.K2_GetActorLocation`))
  (`self.ScheduleNextDrunkSound`))

(event `self.ReceiveBeginPlay`
  (bind _mesh (`self.Mesh`))
  (`SkinnedMeshComponent.SetLeaderPoseComponent` (`self.1_Shirt`) _mesh false false)
  (`SkinnedMeshComponent.SetLeaderPoseComponent` (`self.3_Trousers`) _mesh false false)
  (`SkinnedMeshComponent.SetLeaderPoseComponent` (`self.4_Boots`) _mesh false false)
  (`self.ScheduleNextDrunkSound`))

(event `/Game/LJH/Animations/BPI_HitReaction.RequestHitReaction`
  (params (Attacker :type "Actor Object Reference"))
  (`self.HandleEnemyHitReaction` Attacker))

(fn `UserConstructionScript`)