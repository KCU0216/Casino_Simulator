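; Thief NPC character that steals money from players who walk into its steal trigger.
; On the server, an overlap with a player's capsule asks the game mode to steal money, plays a multicast sound on success, and re-arms after a short delay either way.
; Modular clothing meshes follow the body mesh through leader pose, and hit reaction requests are forwarded to an enemy hit-reaction handler.
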(event `self.ReceiveBeginPlay`
  (bind _mesh (`self.Mesh`))
  (`SkinnedMeshComponent.SetLeaderPoseComponent` (`self.1_Shirt`) _mesh false false)
  (`SkinnedMeshComponent.SetLeaderPoseComponent` (`self.2_Vest`) _mesh false false)
  (`SkinnedMeshComponent.SetLeaderPoseComponent` (`self.3_Trousers`) _mesh false false)
  (`SkinnedMeshComponent.SetLeaderPoseComponent` (`self.4_Boots`) _mesh false false)
  (`SkinnedMeshComponent.SetLeaderPoseComponent` (`self.SkeletalMesh`) _mesh false false))

(event `MC_PlayStealSuccessSound`
  (`CasinoSoundSubsystem.PlaySFX` (subsystem `CasinoSoundSubsystem`) "NPC_Thief_StealSuccess" true (`self.K2_GetActorLocation`)))

(event `self.ReceiveTick`
  (params (DeltaSeconds :type "Float (single-precision)")))

(event `self.StealTrigger.OnComponentBeginOverlap`
  (params (OverlappedComponent :type "PrimitiveComponent Object Reference") (OtherActor :type "Actor Object Reference") (OtherComp :type "PrimitiveComponent Object Reference") (OtherBodyIndex :type Integer) (bFromSweep :type Boolean) (SweepResult :type "HitResult Structure (by ref)"))
  (`/Engine/EditorBlueprintResources/ActorMacros.Switch Has Authority`
    (:`Authority`
      (bind _asbp_first_person_character (cast `/Game/1_BluePrint/Actor/BP_FirstPersonCharacter` OtherActor))
      (if (== OtherComp (`Character.CapsuleComponent` _asbp_first_person_character))
        (`/Engine/EditorBlueprintResources/StandardMacros.DoOnce` false :!label _label
          (:`Completed`
            (bind _ascasino_simulator_game_mode (cast `casino_simulatorGameMode` (`GameplayStatics.GetGameMode`)))
            (bind _returnvalue (`casino_simulatorGameMode.StealMoney` _ascasino_simulator_game_mode _asbp_first_person_character self))
            (if _returnvalue
              (`self.MC_PlayStealSuccessSound`)
              (`KismetSystemLibrary.Delay` 3.0)
              (goto _label :!via `Reset`)
              (else
                (`KismetSystemLibrary.Delay` 3.0)
                (goto _label :!via `Reset`)))))))))

(event `/Game/LJH/Animations/BPI_HitReaction.RequestHitReaction`
  (params (Attacker :type "Actor Object Reference"))
  (`self.HandleEnemyHitReaction` Attacker))

(fn `UserConstructionScript`)