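; Police character that stages an arrival through an entrance door and supports the player jailing and bail flow.
; On arrival it opens the door, then plays a multicast looping walk montage while a timeline lerps it, with sweep, to an exit target.
; Finishing or stopping the encounter ends the montage and resets the door.
; It also supplies the jail destination and activates the bail ATM when a player is jailed.
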(event `Multicast_StopPoliceArrivalWalk`
  (bind _policearrivalwalkmontage (`self.PoliceArrivalWalkMontage`))
  (`/Engine/EditorBlueprintResources/StandardMacros.IsValid` _policearrivalwalkmontage
    (:`Is Valid`
      (`AnimInstance.Montage_Stop` (`SkeletalMeshComponent.GetAnimInstance` (`self.Mesh`)) 0.1 _policearrivalwalkmontage)
      (set `self.PoliceArrivalWalkMontage` null))))

(event `self.ReceiveTick`
  (params (DeltaSeconds :type "Float (single-precision)")))

(event `Multicast_PlayPoliceArrivalWalk`
  (bind _returnvalue (`AnimInstance.PlaySlotAnimationAsDynamicMontage` (`SkeletalMeshComponent.GetAnimInstance` (`self.Mesh`)) "/Game/LJH/Bunny/Dolbani_v2/Animation_v2/AN_Dolbani_Walk.AN_Dolbani_Walk" "DefaultSlot" 0.1 0.1 1.0 100 -1.0 0.0))
  (set `self.PoliceArrivalWalkMontage` _returnvalue))

(event `WalkOutOfDoor`
  (bind _entrancedoor (`self.EntranceDoor`))
  (bind _output_get (set `self.ExitStartLocation` (`self.K2_GetActorLocation`)))
  (bind (_direction _newtrack_0) (`Timeline|TL_PoliceExit` :!via `PlayFromStart` :!label _label)
    (:`Update`
      (`self.K2_SetActorLocationAndRotation` (`KismetMathLibrary.VLerp` _output_get (`self.K2_GetActorLocation` (`self.ExitTarget`)) _newtrack_0) (`self.K2_GetActorRotation`) true))
    (:`Finished`
      (`self.Multicast_StopPoliceArrivalWalk` :!label _label_2)
      (`/Engine/EditorBlueprintResources/StandardMacros.IsValid` _entrancedoor
        (:`Is Valid`
          (`/Game/LJH/Map/BP/BP_Door.ResetDoor` _entrancedoor))))))

(event `self.OnPoliceEncounterStopped`
  (`|ExecutionSequence`
    (:`then_0`
      (goto _label :!via `Stop`))
    (:`then_1`
      (goto _label_2))))

(event `self.OnPoliceArrivalStarted`
  (bind _entrancedoor (`self.EntranceDoor`))
  (add `/Game/LJH/Map/BP/BP_Door.OnDoorOpened` _entrancedoor (delegate `HandleEntranceDoorOpened`))
  (`/Game/LJH/Map/BP/BP_Door.OpenDoor` _entrancedoor))

(event `HandleEntranceDoorOpened`
  (`self.Multicast_PlayPoliceArrivalWalk`)
  (`self.WalkOutOfDoor`))

(event `self.OnPolicePlayerJailed`
  (bind _bailatm (`self.BailATM`))
  (`/Engine/EditorBlueprintResources/StandardMacros.IsValid` _bailatm
    (:`Is Valid`
      (`BailATM.ActivateBailPayment` _bailatm))))

(fn `GetPoliceJailDestination`
  (returns (ReturnValue :type "Actor Object Reference"))
  (return (`self.JailTarget`)))

(fn `UserConstructionScript`)