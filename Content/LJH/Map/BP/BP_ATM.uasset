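; BP_ATM is an ATM actor that drives a linked prison door in response to jail and bail events.
; Its prison-locked, bail-paid and prison-reset events each cast the PrisonDoor reference to BP_Prison_Door and call CloseDoor, OpenDoor or ResetDoor respectively.
; The graph holds only this door forwarding, with no payment logic, and BeginPlay, overlap and Tick are unused.
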(event `self.OnPrisonLocked`
  (bind _asbp_prison_door (cast `/Game/LJH/Map/BP/BP_Prison_Door` (`self.PrisonDoor`)))
  (`/Game/LJH/Map/BP/BP_Prison_Door.CloseDoor` _asbp_prison_door))

(event `self.OnBailPaid`
  (bind _asbp_prison_door (cast `/Game/LJH/Map/BP/BP_Prison_Door` (`self.PrisonDoor`)))
  (`/Game/LJH/Map/BP/BP_Prison_Door.OpenDoor` _asbp_prison_door))

(event `self.OnPrisonReset`
  (bind _asbp_prison_door (cast `/Game/LJH/Map/BP/BP_Prison_Door` (`self.PrisonDoor`)))
  (`/Game/LJH/Map/BP/BP_Prison_Door.ResetDoor` _asbp_prison_door))

(fn `UserConstructionScript`)