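; BP_Prison_Door is a prison door Blueprint that swings a plastic door mesh between closed and open rotations.
; OpenDoor plays a timeline from the start, whose track lerps the mesh's relative rotation to 90 degrees.
; CloseDoor and ResetDoor stop the timeline and snap the mesh instantly, CloseDoor to zero rotation and ResetDoor to the fully open 90-degree rotation.
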(event `self.ReceiveBeginPlay`)

(event `OpenDoor`
  (bind (_direction _newtrack_0) (`Timeline|Timeline` :!via `PlayFromStart` :!label _label)
    (:`Update`
      (`SceneComponent.K2_SetRelativeRotation` (`self.SM_PlasticDoor1`) (`KismetMathLibrary.RLerp` (struct) (struct :`Yaw` 90.0) _newtrack_0) false false))))

(event `CloseDoor`
  (`|ExecutionSequence`
    (:`then_0`
      (goto _label :!via `Stop`))
    (:`then_1`
      (`SceneComponent.K2_SetRelativeRotation` :`self` (`self.SM_PlasticDoor1`)))))

(event `ResetDoor`
  (`|ExecutionSequence`
    (:`then_0`
      (goto _label :!via `Stop`))
    (:`then_1`
      (`SceneComponent.K2_SetRelativeRotation` (`self.SM_PlasticDoor1`) (struct :`Yaw` 90.0) false false))))

(fn `UserConstructionScript`)