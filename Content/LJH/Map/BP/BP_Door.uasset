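; Double door actor that swings its left and right panels open and can be reset to closed.
; OpenDoor plays a timeline from the start, lerping the two panels' relative rotations 90 degrees in opposite directions.
; When the timeline finishes, only the authority calls CallOnDoorOpened.
; ResetDoor stops the timeline and snaps both panels back to zero rotation.
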(event `self.ReceiveBeginPlay`)

(event `OpenDoor`
  (bind (_direction _newtrack_0) (`Timeline|TL_OpenDoor` :!via `PlayFromStart` :!label _label)
    (:`Update`
      (`|ExecutionSequence`
        (:`then_0`
          (`SceneComponent.K2_SetRelativeRotation` (`self.SM_DoorSingleLeft`) (`KismetMathLibrary.RLerp` (struct) (struct :`Yaw` 90.0) _newtrack_0) false false))
        (:`then_1`
          (`SceneComponent.K2_SetRelativeRotation` (`self.SM_DoorSingleRight`) (`KismetMathLibrary.RLerp` (struct) (struct :`Yaw` -90.0) _newtrack_0) false false))))
    (:`Finished`
      (`/Engine/EditorBlueprintResources/ActorMacros.Switch Has Authority`
        (:`Authority`
          (`self.OnDoorOpened`))))))

(event `ResetDoor`
  (`|ExecutionSequence`
    (:`then_0`
      (goto _label :!via `Stop`))
    (:`then_1`
      (`SceneComponent.K2_SetRelativeRotation` :`self` (`self.SM_DoorSingleLeft`))
      (`SceneComponent.K2_SetRelativeRotation` :`self` (`self.SM_DoorSingleRight`)))))

(fn `UserConstructionScript`)