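; Networked 5x3 casino slot machine where a player spends a bet to spin fifteen symbol cylinders for payline wins.
; The server picks a weighted outcome, plants its pattern (or rerolls for a loss), scores it from data tables and multicasts it.
; Lever and reel timelines animate staggered, bouncing stops, then the server pays out and multicasts highlights and popups.
; Machine state gates input and exit; a debug key grants currency.
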(event `self.OnMachineReady`
  (params (RequestingCharacter :type "casino_simulatorCharacter Object Reference"))
  ;[0.15 0.15 0.15 0.5 40] [디버그 전용] - 수정 중
  (set `self.MachineState` "NewEnumerator2")
  (`self.SetCanExitMachine` true)
  (bind _ascasino_simulator_player_controller (cast `casino_simulatorPlayerController` (`Pawn.GetController` RequestingCharacter)))
  (`casino_simulatorPlayerController.SetWorldInteractionPromptControls` _ascasino_simulator_player_controller true true))

(event `self.OnMachinePrimaryInput`
  (params (RequestingCharacter :type "casino_simulatorCharacter Object Reference"))
  ;[0.15 0.15 0.15 0.5 40] [디버그 전용] - 수정 중
  (if (`|EnumEquality` (`self.MachineState`) "NewEnumerator2")
    (`self.SetCanExitMachine` false)
    (bind _ascasino_simulator_player_controller (cast `casino_simulatorPlayerController` (`Pawn.GetController` RequestingCharacter)))
    (`casino_simulatorPlayerController.SetWorldInteractionPromptControls` _ascasino_simulator_player_controller false false)
    (`self.TryStartSpin` RequestingCharacter)))

(event `self.OnMachineReleased`
  (params (ReleasingCharacter :type "casino_simulatorCharacter Object Reference"))
  ;[0.15 0.15 0.15 0.5 40] [디버그 전용] - 수정 중
  (set `self.MachineState` "NewEnumerator0"))

(event `Multicast_StartSpinVisuals`
  (params (ResultSymbols :type "Array of ESlotSymbol Enum") (SpinResult :type "SlotSpinResult Structure"))
  ;[0.15 0.15 0.15 0.5 60] 스핀 요청 및 서버 처리
  ;;[0.15 0.15 0.15 0.5 40] 멀티캐스트 스핀 연출 동기화
  (set `self.CurrentResults` ResultSymbols)
  (set `self.LastSpinResult` SpinResult)
  (`self.ClearWinHighlights`)
  (`self.ShowCurrencyPopup` (* (`self.BetAmount`) -1))
  (`self.StartLeverPull`))

(event `ShowCurrencyPopup`
  (params (Amount :type Integer))
  (bind _currencypopuptext (`self.CurrencyPopupText`))
  (bind _currencypopuptext_2 (`self.CurrencyPopupText`))
  ;[0.15 0.15 0.15 0.5 60] 화면 표시 및 팝업 처리
  ;;[0.15 0.15 0.15 0.5 40] 금액 변동 팝업 표시
  (if (!= Amount 0)
    (if (> Amount 0)
      (`TextRenderComponent.K2_SetText` _currencypopuptext (`KismetTextLibrary.Conv_StringToText` (`KismetStringLibrary.Concat_StrStr` "+" (`KismetStringLibrary.Conv_IntToString` Amount))))
      (`TextRenderComponent.SetTextRenderColor` _currencypopuptext (`KismetMathLibrary.Conv_LinearColorToColor` (make `LinearColor` 1.0 0.75 0.0 1.0)))
      (`SceneComponent.SetHiddenInGame` _currencypopuptext false false)
      (`KismetSystemLibrary.K2_SetTimer` null "HideCurrencyPopup" 1.5)
      (else
        (`TextRenderComponent.K2_SetText` _currencypopuptext_2 (`KismetTextLibrary.Conv_StringToText` (`KismetStringLibrary.Concat_StrStr` "-" (`KismetStringLibrary.Conv_IntToString` (`KismetMathLibrary.Abs_Int` Amount)))))
        (`TextRenderComponent.SetTextRenderColor` _currencypopuptext_2 (`KismetMathLibrary.Conv_LinearColorToColor` (make `LinearColor` 1.0 0.05 0.02 1.0)))
        (`SceneComponent.SetHiddenInGame` _currencypopuptext_2 false false)
        (`KismetSystemLibrary.K2_SetTimer` null "HideCurrencyPopup" 1.0)))))

(event `TryStartSpin`
  (params (RequestingCharacter :type "casino_simulatorCharacter Object Reference"))
  ;[0.15 0.15 0.15 0.5 60] 스핀 요청 및 서버 처리
  ;;[0.15 0.15 0.15 0.5 40] 스핀 요청 서버 전달
  (`self.Server_TryStartSpin` RequestingCharacter))

(event `Multicast_ShowResultVisuals`
  (params (SpinResult :type "SlotSpinResult Structure"))
  ;[0.15 0.15 0.15 0.5 60] 스핀 요청 및 서버 처리
  ;;[0.15 0.15 0.15 0.5 40] 멀티캐스트 결과 연출 동기화
  (bind _output_get (set `self.LastSpinResult` SpinResult))
  (`self.ShowWinHighlights` _output_get)
  (bind (_biswin _bisfullscreen _resulttype _winningsymbol _bestmatchcount _totalrewardamount) (break `SlotSpinResult` _output_get))
  (if (> _totalrewardamount 0)
    (`self.ShowCurrencyPopup` _totalrewardamount))
  (`KismetSystemLibrary.K2_SetTimerDelegate` (delegate `ClearResultHighlightsDelayed`) 1.5))

(event `ClearResultHighlightsDelayed`
  ;[0.15 0.15 0.15 0.5 60] 스핀 요청 및 서버 처리
  ;;[0.15 0.15 0.15 0.5 40] 멀티캐스트 결과 연출 동기화
  (`self.ClearWinHighlights`))

(event `Key|U`
  (params (Key :type "Key Structure"))
  ;[0.15 0.15 0.15 0.5 60] [디버그 전용]
  ;;[0.15 0.15 0.15 0.5 40] [디버그 전용] 테스트 금액 지급 -
  ;; 정식 경제 시스템 연결 전까지 유지
  (:`Pressed`
    (bind _ascasino_simulator_character (cast `casino_simulatorCharacter` (`GameplayStatics.GetPlayerCharacter` 0)))
    (`casino_simulatorCharacter.AddCurrency` _ascasino_simulator_character 1000.0)
    (`KismetSystemLibrary.PrintString` (`KismetStringLibrary.Conv_DoubleToString` (`casino_simulatorCharacter.GetCurrency` _ascasino_simulator_character)))))

(event `HideCurrencyPopup`
  ;[0.15 0.15 0.15 0.5 60] 화면 표시 및 팝업 처리
  ;;[0.15 0.15 0.15 0.5 40] 금액 팝업 숨김
  (`SceneComponent.SetHiddenInGame` (`self.CurrencyPopupText`) true false))

(event `Server_TryStartSpin`
  (params (RequestingCharacter :type "casino_simulatorCharacter Object Reference"))
  (bind _machinestate (`self.MachineState`))
  (bind _currentresults (`self.CurrentResults`))
  ;[0.15 0.15 0.15 0.5 60] 스핀 요청 및 서버 처리
  ;;[0.15 0.15 0.15 0.5 40] 서버 권한 스핀 처리
  (if (`self.CanOperate` RequestingCharacter)
    (if (not (or (`|EnumEquality` _machinestate "NewEnumerator3") (`|EnumEquality` _machinestate "NewEnumerator4") (`|EnumEquality` _machinestate "NewEnumerator5")))
      (bind _returnvalue (`casino_simulatorCharacter.TrySpendCurrency` RequestingCharacter (`KismetMathLibrary.Conv_IntToDouble` (`self.BetAmount`))))
      (if _returnvalue
        (`self.GenerateResults`)
        (bind _output_get (set `self.LastSpinResult` (`SlotMachineBlueprintLibrary.EvaluateSlotResultWithPayout` _currentresults (`self.SymbolDataTable`) (`self.PayoutDataTable `) (`self.BetAmount`))))
        (`self.Multicast_StartSpinVisuals` _currentresults _output_get)
        (else
          (set `self.MachineState` "NewEnumerator2")
          (`self.SetCanExitMachine` true)
          (bind _ascasino_simulator_player_controller (cast `casino_simulatorPlayerController` (`Pawn.GetController` RequestingCharacter)))
          (`casino_simulatorPlayerController.SetWorldInteractionPromptControls` _ascasino_simulator_player_controller true true)
          (`KismetSystemLibrary.PrintString` "\"잔액이 부족합니다.\""))))))

(event `self.ReceiveBeginPlay`
  ;[0.15 0.15 0.15 0.5 60] [디버그 전용]
  ;;[0.15 0.15 0.15 0.5 30] [디버그 전용]  입력 활성화 및 하이라이트 초기화
  (`|ExecutionSequence`
    (:`then_0`
      (`self.InitializeHighlightBorders`))
    (:`then_1`
      (`/Engine/EditorBlueprintResources/ActorMacros.Switch Has Authority`
        (:`Authority`
          (set `self.MachineState` "NewEnumerator2"))))))

(event `StartLeverPull`
  (bind _lastspinresult (`self.LastSpinResult`))
  (bind (_biswin _bisfullscreen _resulttype _winningsymbol _bestmatchcount _totalrewardamount) (break `SlotSpinResult` _lastspinresult))
  ;[0.15 0.15 0.15 0.5 60] 릴 회전 및 결과 처리
  ;;[0.15 0.15 0.15 0.5 40] 레버 연출 시작
  (set `self.MachineState` "NewEnumerator3")
  (bind (_direction _leveralpha) (`Timeline|TL_LeverPull` :!via `PlayFromStart`)
    (:`Update`
      (`self.ApplyLeverAngle` (`KismetMathLibrary.Lerp` (`self.LeverUpAngleX`) (`self.LeverDownAngleX`) _leveralpha)))
    (:`StartReels`
      ;;[0.15 0.15 0.15 0.5 40] 동기화된 결과로 릴 회전 준비
      (set `self.MachineState` "NewEnumerator4")
      (`|ExecutionSequence`
        (:`then_0`
          (`self.BuildTargetAngles`)
          (`self.PrepareReelSpin`)
          (bind (_direction_2 _spinelapsed) (`Timeline|TL_ReelSpin` :!via `PlayFromStart`)
            (:`Update`
              ;;[0.15 0.15 0.15 0.5 40] 릴 회전 업데이트 및 서버 정산
              (`self.UpdateReelSpin` _spinelapsed))
            (:`Finished`
              (`self.SnapReelsToTargetAngles`)
              (`/Engine/EditorBlueprintResources/ActorMacros.Switch Has Authority`
                (:`Authority`
                  (if (> _totalrewardamount 0)
                    (`casino_simulatorCharacter.AddCurrency` (`self.GetCurrentUser`) (`KismetMathLibrary.Conv_IntToDouble` _totalrewardamount)))
                  (`self.Multicast_ShowResultVisuals` _lastspinresult)
                  (set `self.MachineState` "NewEnumerator5")
                  (`KismetSystemLibrary.K2_SetTimerDelegate` (delegate `ResetMachineStateAfterResult`) 0.2))))))
        (:`then_1`
          ;;[0.15 0.15 0.15 0.5 40] 디버그 - 당첨 라인 로그 출력
          (for _array_element (`.LineWins` (break `SlotSpinResult` (`self.LastSpinResult`)))
            (bind (_lineindex _linetype _lineindexes _winningsymbol_2 _resulttype_2 _rewardtype _matchcount _symbolmultiplier _resultmultiplier _rewardamount) (break `SlotLineWin` _array_element))
            (`KismetSystemLibrary.PrintString` (`KismetTextLibrary.Conv_TextToString` (`|FormatText` "Line {LineIndex} / {LineType} / {Symbol} / Count {Count} / Reward {Reward}" _lineindex (`|GetEnumeratorNameAsString` _linetype) (`KismetTextLibrary.Conv_StringToText` (`KismetStringLibrary.Conv_NameToString` (`SlotMachineBlueprintLibrary.GetSlotSymbolRowName` _winningsymbol_2))) _matchcount _rewardamount)))))))))

(event `ResetMachineStateAfterResult`
  ;[0.15 0.15 0.15 0.5 60] 릴 회전 및 결과 처리
  ;;[0.15 0.15 0.15 0.5 40] 릴 회전 업데이트 및 서버 정산
  (set `self.MachineState` "NewEnumerator2")
  (`self.SetCanExitMachine` true)
  (bind _ascasino_simulator_player_controller (cast `casino_simulatorPlayerController` (`Pawn.GetController` (`self.GetCurrentUser`))))
  (`casino_simulatorPlayerController.SetWorldInteractionPromptControls` _ascasino_simulator_player_controller true true))

(fn `ApplyLeverAngle`
  (params (AngleX :type "Float (double-precision)"))
  (bind _sm_lever_handle_hub (`self.SM_Lever_Handle_Hub`))
  ;[0.15 0.15 0.15 0.5 40] 레버 X축 회전 적용
  (`SceneComponent.K2_SetRelativeRotation` _sm_lever_handle_hub (`KismetMathLibrary.MakeRotator` AngleX (.pitch (`SceneComponent.RelativeRotation` _sm_lever_handle_hub)) (.yaw (`SceneComponent.RelativeRotation` _sm_lever_handle_hub))) false false))

(fn `ApplyReelAngle`
  (params (AngleX :type "Float (double-precision)") (ReelIndex :type Integer))
  (bind _reelcomponents (`self.ReelComponents`))
  (bind _output (`|GetArrayItem` _reelcomponents ReelIndex))
  ;[0.15 0.15 0.15 0.5 40] 릴 인덱스 검증 및 X축 회전 적용
  (if (`KismetArrayLibrary.Array_IsValidIndex` _reelcomponents ReelIndex)
    (`SceneComponent.K2_SetRelativeRotation` _output (`KismetMathLibrary.MakeRotator` AngleX (.pitch (`SceneComponent.RelativeRotation` _output)) (.yaw (`SceneComponent.RelativeRotation` _output))) false false)))

(fn `BuildTargetAngles`
  ;[0.15 0.15 0.15 0.5 40] 결과 심볼별 목표 각도 배열 생성
  (`KismetArrayLibrary.Array_Clear` (`self.TargetAngles`))
  (for _array_element (`self.CurrentResults`)
    (bind _returnvalue (`|GetDataTableRow` (`self.SymbolDataTable`) (`SlotMachineBlueprintLibrary.GetSlotSymbolRowName` _array_element))
      (:`then`
        (`KismetArrayLibrary.Array_Add` (`self.TargetAngles`) (`.TargetAngleX` (break `SlotSymbolData` _returnvalue))))
      (:`RowNotFound`
        (`KismetSystemLibrary.PrintString` "Symbol row not found")
        (`KismetArrayLibrary.Array_Add` (`self.TargetAngles`))))))

(fn `CalculateFinalReelAngle`
  (params (TargetAngle :type "Float (double-precision)") (CurrentAngle :type "Float (double-precision)") (ExtraTurns :type Integer))
  (returns (FinalAngle :type "Float (double-precision)"))
  ;[0.15 0.15 0.15 0.5 30] 최종 릴 정지 각도 계산
  (return (+ (`KismetMathLibrary.ClampAxis` (- TargetAngle (`KismetMathLibrary.ClampAxis` CurrentAngle))) (+ CurrentAngle (* ExtraTurns 360)))))

(fn `ClearWinHighlights`
  (for _array_element (`self.ReelHighlightBorders`)
    (`/Engine/EditorBlueprintResources/StandardMacros.IsValid` _array_element
      (:`Is Valid`
        (`SceneComponent.SetHiddenInGame` _array_element true false)))))

(fn `GenerateRandomBaseResults`
  (bind _currentresults (`self.CurrentResults`))
  (bind _allsymbols (`self.AllSymbols`))
  ;[0.15 0.15 0.15 0.5 40] 기본 15칸 랜덤 결과 생성
  (`KismetArrayLibrary.Array_Clear` _currentresults)
  (for _ (range 15)
    (`KismetArrayLibrary.Array_Add` _currentresults (`|GetArrayItem` _allsymbols (`KismetMathLibrary.RandomIntegerInRange` 0 (- (`KismetArrayLibrary.Array_Length` _allsymbols) 1))))))

(fn `GenerateResults`
  ;[0.15 0.15 0.15 0.5 40] 결과 생성 흐름 제어
  (`self.GenerateRandomBaseResults`)
  (bind _output_get (set `self.SelectedOutcome` (`SlotMachineBlueprintLibrary.RollSpinOutcomeByWeight` (`self.OutcomeWeightDataTable`))))
  (switch `ESlotSpinOutcome` _output_get
    (:`Lose`
      ;[0.15 0.15 0.15 0.5 40] Lose 방어 - 당첨 없는 배열 재생성
      (for _ (range 51)
        (`self.GenerateRandomBaseResults`)
        (if (== (`.bIsWin` (break `SlotSpinResult` (`SlotMachineBlueprintLibrary.EvaluateSlotResult` (`self.CurrentResults`)))) false)
          (break))))
    (:`Horizontal3`
      ;[0.15 0.15 0.15 0.5 40] 목표 족보 심기 - Horizontal3
      ;; 당첨 심볼 확정
      (bind _output_get_2 (set `self.TempWinningSymbol` (`|GetArrayItem` (`self.AllSymbols`) (`KismetMathLibrary.RandomIntegerInRange` 0 (- (`KismetArrayLibrary.Array_Length` (`self.AllSymbols`)) 1)))))
      ;; 당첨 라인 확정
      (bind _output_get_3 (set `self.TempLineIndexes` (`SlotMachineBlueprintLibrary.GetPaylineIndexes` (`KismetMathLibrary.RandomIntegerInRange` 0 2))))
      ;; 확정된 심볼을 확정된 라인에 랜덤배열로 배치
      (bind _output_get_4 (set `self.TempStartOffset` (`KismetMathLibrary.RandomIntegerInRange` 0 2)))
      (for _index (range 3)
        (`KismetArrayLibrary.Array_Set` (`self.CurrentResults`) (`|GetArrayItem` _output_get_3 (+ _index _output_get_4)) _output_get_2)))
    (:`Horizontal4`
      ;[0.15 0.15 0.15 0.5 40] 목표 족보 심기 - Horizontal4
      ;; 당첨 심볼 확정
      (bind _output_get_5 (set `self.TempWinningSymbol` (`|GetArrayItem` (`self.AllSymbols`) (`KismetMathLibrary.RandomIntegerInRange` 0 (- (`KismetArrayLibrary.Array_Length` (`self.AllSymbols`)) 1)))))
      ;; 당첨 라인 확정
      (bind _output_get_6 (set `self.TempLineIndexes` (`SlotMachineBlueprintLibrary.GetPaylineIndexes` (`KismetMathLibrary.RandomIntegerInRange` 0 2))))
      ;; 확정된 심볼을 확정된 라인에 랜덤배열로 배치
      (bind _output_get_7 (set `self.TempStartOffset` (`KismetMathLibrary.RandomIntegerInRange` 0 1)))
      (for _index_2 (range 4)
        (`KismetArrayLibrary.Array_Set` (`self.CurrentResults`) (`|GetArrayItem` _output_get_6 (+ _index_2 _output_get_7)) _output_get_5)))
    (:`Horizontal5`
      ;[0.15 0.15 0.15 0.5 40] 목표 족보 심기 - Horizontal5
      ;; 당첨 심볼 확정
      (bind _output_get_8 (set `self.TempWinningSymbol` (`|GetArrayItem` (`self.AllSymbols`) (`KismetMathLibrary.RandomIntegerInRange` 0 (- (`KismetArrayLibrary.Array_Length` (`self.AllSymbols`)) 1)))))
      ;; 당첨 라인 확정
      (bind _output_get_9 (set `self.TempLineIndexes` (`SlotMachineBlueprintLibrary.GetPaylineIndexes` (`KismetMathLibrary.RandomIntegerInRange` 0 2))))
      ;; 확정된 심볼을 확정된 라인에 랜덤배열로 배치
      (bind _output_get_10 (set `self.TempStartOffset` (`KismetMathLibrary.RandomIntegerInRange` 0)))
      (for _index_3 (range 5)
        (`KismetArrayLibrary.Array_Set` (`self.CurrentResults`) (`|GetArrayItem` _output_get_9 (+ _index_3 _output_get_10)) _output_get_8)))
    (:`Vertical3`
      ;[0.15 0.15 0.15 0.5 40] 목표 족보 심기 - Vertical3
      ;; 당첨 심볼 확정
      (bind _output_get_11 (set `self.TempWinningSymbol` (`|GetArrayItem` (`self.AllSymbols`) (`KismetMathLibrary.RandomIntegerInRange` 0 (- (`KismetArrayLibrary.Array_Length` (`self.AllSymbols`)) 1)))))
      ;; 당첨 라인 확정
      (bind _output_get_12 (set `self.TempLineIndexes` (`SlotMachineBlueprintLibrary.GetPaylineIndexes` (`KismetMathLibrary.RandomIntegerInRange` 5 9))))
      ;; 확정된 심볼을 확정된 라인에 배치
      (for _index_4 (range 3)
        (`KismetArrayLibrary.Array_Set` (`self.CurrentResults`) (`|GetArrayItem` _output_get_12 _index_4) _output_get_11)))
    (:`Diagonal3`
      ;[0.15 0.15 0.15 0.5 40] 목표 족보 심기 - Diagonal3
      ;; 당첨 심볼 확정
      (bind _output_get_13 (set `self.TempWinningSymbol` (`|GetArrayItem` (`self.AllSymbols`) (`KismetMathLibrary.RandomIntegerInRange` 0 (- (`KismetArrayLibrary.Array_Length` (`self.AllSymbols`)) 1)))))
      ;; 당첨 라인 확정
      (bind _output_get_14 (set `self.TempLineIndexes` (`SlotMachineBlueprintLibrary.GetPaylineIndexes` (`KismetMathLibrary.RandomIntegerInRange` 10 15))))
      ;; 확정된 심볼을 확정된 라인에 배치
      (for _index_5 (range 3)
        (`KismetArrayLibrary.Array_Set` (`self.CurrentResults`) (`|GetArrayItem` _output_get_14 _index_5) _output_get_13)))
    (:`VShape5`
      ;[0.15 0.15 0.15 0.5 40] 목표 족보 심기 - VShape5
      ;; 당첨 심볼 확정
      (bind _output_get_15 (set `self.TempWinningSymbol` (`|GetArrayItem` (`self.AllSymbols`) (`KismetMathLibrary.RandomIntegerInRange` 0 (- (`KismetArrayLibrary.Array_Length` (`self.AllSymbols`)) 1)))))
      ;; 당첨 라인 확정
      (bind _output_get_16 (set `self.TempLineIndexes` (`SlotMachineBlueprintLibrary.GetPaylineIndexes` 3)))
      ;; 확정된 심볼을 확정된 라인에 배치
      (for _index_6 (range 5)
        (`KismetArrayLibrary.Array_Set` (`self.CurrentResults`) (`|GetArrayItem` _output_get_16 _index_6) _output_get_15)))
    (:`InvertedVShape5`
      ;[0.15 0.15 0.15 0.5 40] 목표 족보 심기 - InvertedVShape5
      ;; 당첨 심볼 확정
      (bind _output_get_17 (set `self.TempWinningSymbol` (`|GetArrayItem` (`self.AllSymbols`) (`KismetMathLibrary.RandomIntegerInRange` 0 (- (`KismetArrayLibrary.Array_Length` (`self.AllSymbols`)) 1)))))
      ;; 당첨 라인 확정
      (bind _output_get_18 (set `self.TempLineIndexes` (`SlotMachineBlueprintLibrary.GetPaylineIndexes` 4)))
      ;; 확정된 심볼을 확정된 라인에 배치
      (for _index_7 (range 5)
        (`KismetArrayLibrary.Array_Set` (`self.CurrentResults`) (`|GetArrayItem` _output_get_18 _index_7) _output_get_17)))
    (:`FullScreen`
      ;[0.15 0.15 0.15 0.5 40] 목표 족보 심기 - FullScreen
      ;; 당첨 심볼 확정
      (bind _output_get_19 (set `self.TempWinningSymbol` (`|GetArrayItem` (`self.AllSymbols`) (`KismetMathLibrary.RandomIntegerInRange` 0 (- (`KismetArrayLibrary.Array_Length` (`self.AllSymbols`)) 1)))))
      ;; 확정된 심볼을 배치
      (for _index_8 (range 15)
        (`KismetArrayLibrary.Array_Set` (`self.CurrentResults`) _index_8 _output_get_19)))))

(fn `InitializeHighlightBorders`
  (set `self.ReelHighlightBorders` (`|MakeArray` (`self.HL_01`) (`self.HL_02`) (`self.HL_03`) (`self.HL_04`) (`self.HL_05`) (`self.HL_06`) (`self.HL_07`) (`self.HL_08`) (`self.HL_09`) (`self.HL_10`) (`self.HL_11`) (`self.HL_12`) (`self.HL_13`) (`self.HL_14`) (`self.HL_15`)))
  (`self.ClearWinHighlights`))

(fn `PrepareReelSpin`
  ;[0.15 0.15 0.15 0.5 40] 릴별 시작 및 최종 회전 각도 계산
  (`KismetArrayLibrary.Array_Clear` (`self.StartAngles`))
  (`KismetArrayLibrary.Array_Clear` (`self.FinalAngles`))
  (`KismetArrayLibrary.Array_Clear` (`self.ReelStopTimes`))
  (for (_array_element _array_index) (`self.ReelComponents`)
    (bind _roll (.roll (`SceneComponent.RelativeRotation` _array_element)))
    (`KismetArrayLibrary.Array_Add` (`self.StartAngles`) _roll)
    (`KismetArrayLibrary.Array_Add` (`self.FinalAngles`) (`self.CalculateFinalReelAngle` (`|GetArrayItem` (`self.TargetAngles`) _array_index) _roll (+ _array_index 3)))
    (`KismetArrayLibrary.Array_Add` (`self.ReelStopTimes`) (+ (* _array_index 0.2) 0.7))))

(fn `ShowWinHighlights`
  (params (SpinResult :type "SlotSpinResult Structure"))
  (`self.ClearWinHighlights`)
  (for _array_element (`.LineWins` (break `SlotSpinResult` SpinResult))
    (for _array_element_2 (`.LineIndexes` (break `SlotLineWin` _array_element))
      (bind _output (`|GetArrayItem` (`self.ReelHighlightBorders`) _array_element_2))
      (`/Engine/EditorBlueprintResources/StandardMacros.IsValid` _output
        (:`Is Valid`
          (`SceneComponent.SetHiddenInGame` _output false false)))))
  (`KismetSystemLibrary.K2_SetTimer` null "ClearWinHighlights" 2.0))

(fn `SnapReelsToTargetAngles`
  ;[0.15 0.15 0.15 0.5 30] 모든 릴을 목표 각도로 최종 보정
  (for (_array_element _array_index) (`self.TargetAngles`)
    (`self.ApplyReelAngle` _array_element _array_index)))

(fn `UpdateReelSpin`
  (params (ElapsedTime :type "Float (double-precision)"))
  (locals (CurrentReelAngle :type "Float (double-precision)"))
  ;[0.15 0.15 0.15 0.5 40] 릴 회전 감속 및 정지 바운스 적용
  (for (_array_element _array_index) (`self.StartAngles`)
    (bind _output (`|GetArrayItem` (`self.ReelStopTimes`) _array_index))
    (bind _output_get (set `local.CurrentReelAngle` (`|EaseFunction` "Linear" (`KismetMathLibrary.MapRangeClamped` ElapsedTime 0.0 _output 0.0 1.0) _array_element (`|GetArrayItem` (`self.FinalAngles`) _array_index))))
    (`self.ApplyReelAngle` (+ _output_get (`CurveFloat.GetFloatValue` (`self.WeakReelBounceCurve`) (- ElapsedTime _output))) _array_index)))

(fn `UserConstructionScript`
  ;[0.15 0.15 0.15 0.5 30] 릴 컴포넌트 배열 초기화
  (set `self.ReelComponents` (`|MakeArray` (`self.SM_Reel_05_Cylinder1`) (`self.SM_Reel_05_Cylinder2`) (`self.SM_Reel_05_Cylinder3`) (`self.SM_Reel_05_Cylinder4`) (`self.SM_Reel_05_Cylinder5`) (`self.SM_Reel_05_Cylinder6`) (`self.SM_Reel_05_Cylinder7`) (`self.SM_Reel_05_Cylinder8`) (`self.SM_Reel_05_Cylinder9`) (`self.SM_Reel_05_Cylinder10`) (`self.SM_Reel_05_Cylinder11`) (`self.SM_Reel_05_Cylinder12`) (`self.SM_Reel_05_Cylinder13`) (`self.SM_Reel_05_Cylinder14`) (`self.SM_Reel_05_Cylinder15`))))