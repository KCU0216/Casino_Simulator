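; Three Card Poker table actor that shows dealt hands as animated cards and opens the betting UI on the interacting first-person character.
; Deal events fill three child-actor slots per side in order, reusing BP_BlackjackCard and its visuals DataTable.
; Player cards fly face-up from DeckPoint, while dealer cards fly from ViewPoint using each card's face-up flag.
; The reveal event turns dealer cards face-up, and table changes at round state 0 hide all cards.
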(event `self.ReceiveBeginPlay`
  (add `self.OnPlayerCardDealt` (delegate `OnPlayerCardDealt_이벤트`))
  (add `self.OnDealerCardDealt` (delegate `OnDealerCardDealt_이벤트`))
  (add `self.OnDealerHandRevealed` (delegate `OnDealerHandRevealed_이벤트`))
  (add `self.OnTableChanged` (delegate `OnTableChanged_이벤트`))
  (`self.ResetThreeCardPokerCardVisuals`))

(event `OnPlayerCardDealt_이벤트` :!signature `self.OnPlayerCardDealt`
  (params (Card :type "BlackjackCard Structure (by ref)"))
  (`self.DealVisualCardToPlayer` Card))

(event `OnDealerCardDealt_이벤트` :!signature `self.OnDealerCardDealt`
  (params (Card :type "BlackjackCard Structure (by ref)"))
  (`self.DealVisualCardToDealer` Card))

(event `OnDealerHandRevealed_이벤트`
  (`self.RevealDealerHandVisual`))

(event `OnTableChanged_이벤트`
  (if (== (`self.GetRoundState`) 0)
    (`self.ResetThreeCardPokerCardVisuals`)))

(event `self.OnLocalInteract`
  (params (InteractingCharacter :type "casino_simulatorCharacter Object Reference"))
  (bind _asbp_first_person_character (cast `/Game/1_BluePrint/Actor/BP_FirstPersonCharacter` InteractingCharacter))
  (bind _output_get (set `self.As BP First Person Character` _asbp_first_person_character))
  (`/Game/1_BluePrint/Actor/BP_FirstPersonCharacter.OpenThreeCardPokerBetting` _output_get))

(fn `DealVisualCardToDealer`
  (params (Card :type "BlackjackCard Structure"))
  (bind (_suit _rank _bfaceup) (break `BlackjackCard` Card))
  (bind _nextdealercardindex (`self.NextDealerCardIndex`))
  (bind _dealercard0 (`self.DealerCard0`))
  (bind _dealercard1 (`self.DealerCard1`))
  (bind _dealercard2 (`self.DealerCard2`))
  (bind (_deckstyle _suit_2 _rank_2 _fronttexture _backtexture) (break `BlackjackCardVisualData` (`BlackjackBlueprintLibrary.FindBlackjackCardVisualData` "/Game/Blackjack/Data/DT_BlackjackCardVisuals.DT_BlackjackCardVisuals" "CasinoRed" Card)))
  (bind _returnvalue_location (`KismetMathLibrary.BreakTransform` (`SceneComponent.K2_GetComponentToWorld` _dealercard2)))
  (bind _returnvalue_location_2 (`KismetMathLibrary.BreakTransform` (`SceneComponent.K2_GetComponentToWorld` _dealercard0)))
  (bind _returnvalue_location_3 (`KismetMathLibrary.BreakTransform` (`SceneComponent.K2_GetComponentToWorld` _dealercard1)))
  (bind _childactor (`ChildActorComponent.ChildActor` _dealercard0))
  (bind _childactor_2 (`ChildActorComponent.ChildActor` _dealercard1))
  (bind _childactor_3 (`ChildActorComponent.ChildActor` _dealercard2))
  (bind _location (.location (`SceneComponent.K2_GetComponentToWorld` (`self.ViewPoint`))))
  (bind _rotation (.rotation (`SceneComponent.K2_GetComponentToWorld` (`self.ViewPoint`))))
  (if (== _nextdealercardindex 0)
    (`self.SetActorHiddenInGame` _childactor false)
    (bind _asbp_blackjack_card (cast `/Game/Blackjack/BluePrint/Card/BP_BlackjackCard` _childactor))
    (`self.K2_SetActorLocationAndRotation` _asbp_blackjack_card _location _rotation false true)
    (`/Game/Blackjack/BluePrint/Card/BP_BlackjackCard.InitializeCard` _asbp_blackjack_card _fronttexture _backtexture _bfaceup)
    (`/Game/Blackjack/BluePrint/Card/BP_BlackjackCard.DealTo` _asbp_blackjack_card (`KismetMathLibrary.MakeTransform` _returnvalue_location_2 (struct :`Pitch` 180.0 :`Roll` -90.0) (10.0 10.0 10.0)) 0.6 false)
    (elif (== _nextdealercardindex 1)
      (`self.SetActorHiddenInGame` _childactor_2 false)
      (bind _asbp_blackjack_card_2 (cast `/Game/Blackjack/BluePrint/Card/BP_BlackjackCard` _childactor_2))
      (`self.K2_SetActorLocationAndRotation` _asbp_blackjack_card_2 _location _rotation false true)
      (`/Game/Blackjack/BluePrint/Card/BP_BlackjackCard.InitializeCard` _asbp_blackjack_card_2 _fronttexture _backtexture _bfaceup)
      (`/Game/Blackjack/BluePrint/Card/BP_BlackjackCard.DealTo` _asbp_blackjack_card_2 (`KismetMathLibrary.MakeTransform` _returnvalue_location_3 (struct :`Pitch` 180.0 :`Roll` -90.0) (10.0 10.0 10.0)) 0.6 false)
      (else
        (`self.SetActorHiddenInGame` _childactor_3 false)
        (bind _asbp_blackjack_card_3 (cast `/Game/Blackjack/BluePrint/Card/BP_BlackjackCard` _childactor_3))
        (`self.K2_SetActorLocationAndRotation` _asbp_blackjack_card_3 _location _rotation false true)
        (`/Game/Blackjack/BluePrint/Card/BP_BlackjackCard.InitializeCard` _asbp_blackjack_card_3 _fronttexture _backtexture _bfaceup)
        (`/Game/Blackjack/BluePrint/Card/BP_BlackjackCard.DealTo` _asbp_blackjack_card_3 (`KismetMathLibrary.MakeTransform` _returnvalue_location (struct :`Pitch` 180.0 :`Roll` -90.0) (10.0 10.0 10.0)) 0.6 false))))
  (set `self.NextDealerCardIndex` (+ _nextdealercardindex 1)))

(fn `DealVisualCardToPlayer`
  (params (Card :type "BlackjackCard Structure"))
  (bind _nextplayercardindex (`self.NextPlayerCardIndex`))
  (bind _playercard0 (`self.PlayerCard0`))
  (bind _playercard1 (`self.PlayerCard1`))
  (bind _playercard2 (`self.PlayerCard2`))
  (bind (_deckstyle _suit _rank _fronttexture _backtexture) (break `BlackjackCardVisualData` (`BlackjackBlueprintLibrary.FindBlackjackCardVisualData` "/Game/Blackjack/Data/DT_BlackjackCardVisuals.DT_BlackjackCardVisuals" "CasinoRed" Card)))
  (bind (_returnvalue_location _returnvalue_rotation _returnvalue_scale) (`KismetMathLibrary.BreakTransform` (`SceneComponent.K2_GetComponentToWorld` _playercard2)))
  (bind (_returnvalue_location_2 _returnvalue_rotation_2 _returnvalue_scale_2) (`KismetMathLibrary.BreakTransform` (`SceneComponent.K2_GetComponentToWorld` _playercard0)))
  (bind (_returnvalue_location_3 _returnvalue_rotation_3 _returnvalue_scale_3) (`KismetMathLibrary.BreakTransform` (`SceneComponent.K2_GetComponentToWorld` _playercard1)))
  (bind _childactor (`ChildActorComponent.ChildActor` _playercard0))
  (bind _childactor_2 (`ChildActorComponent.ChildActor` _playercard1))
  (bind _childactor_3 (`ChildActorComponent.ChildActor` _playercard2))
  (bind _location (.location (`SceneComponent.K2_GetComponentToWorld` (`self.DeckPoint`))))
  (bind _rotation (.rotation (`SceneComponent.K2_GetComponentToWorld` (`self.DeckPoint`))))
  (if (== _nextplayercardindex 0)
    (`self.SetActorHiddenInGame` _childactor false)
    (bind _asbp_blackjack_card (cast `/Game/Blackjack/BluePrint/Card/BP_BlackjackCard` _childactor))
    (`self.K2_SetActorLocationAndRotation` _asbp_blackjack_card _location _rotation false true)
    (`/Game/Blackjack/BluePrint/Card/BP_BlackjackCard.InitializeCard` _asbp_blackjack_card _fronttexture _backtexture true)
    (`/Game/Blackjack/BluePrint/Card/BP_BlackjackCard.DealTo` _asbp_blackjack_card (`KismetMathLibrary.MakeTransform` _returnvalue_location_2 (struct :`Pitch` 180.0 :`Roll` -90.0) _returnvalue_scale_2) 0.6 true)
    (elif (== _nextplayercardindex 1)
      (`self.SetActorHiddenInGame` _childactor_2 false)
      (bind _asbp_blackjack_card_2 (cast `/Game/Blackjack/BluePrint/Card/BP_BlackjackCard` _childactor_2))
      (`self.K2_SetActorLocationAndRotation` _asbp_blackjack_card_2 _location _rotation false true)
      (`/Game/Blackjack/BluePrint/Card/BP_BlackjackCard.InitializeCard` _asbp_blackjack_card_2 _fronttexture _backtexture true)
      (`/Game/Blackjack/BluePrint/Card/BP_BlackjackCard.DealTo` _asbp_blackjack_card_2 (`KismetMathLibrary.MakeTransform` _returnvalue_location_3 (struct :`Pitch` 180.0 :`Roll` -90.0) _returnvalue_scale_3) 0.6 true)
      (else
        (`self.SetActorHiddenInGame` _childactor_3 false)
        (bind _asbp_blackjack_card_3 (cast `/Game/Blackjack/BluePrint/Card/BP_BlackjackCard` _childactor_3))
        (`self.K2_SetActorLocationAndRotation` _asbp_blackjack_card_3 _location _rotation false true)
        (`/Game/Blackjack/BluePrint/Card/BP_BlackjackCard.InitializeCard` _asbp_blackjack_card_3 _fronttexture _backtexture true)
        (`/Game/Blackjack/BluePrint/Card/BP_BlackjackCard.DealTo` _asbp_blackjack_card_3 (`KismetMathLibrary.MakeTransform` _returnvalue_location (struct :`Pitch` 180.0 :`Roll` -90.0) _returnvalue_scale) 0.6 true))))
  (set `self.NextPlayerCardIndex` (+ _nextplayercardindex 1)))

(fn `ResetThreeCardPokerCardVisuals`
  (`self.SetActorHiddenInGame` (`ChildActorComponent.ChildActor` (`self.PlayerCard0`)) true)
  (`self.SetActorHiddenInGame` (`ChildActorComponent.ChildActor` (`self.PlayerCard1`)) true)
  (`self.SetActorHiddenInGame` (`ChildActorComponent.ChildActor` (`self.PlayerCard2`)) true)
  (`self.SetActorHiddenInGame` (`ChildActorComponent.ChildActor` (`self.DealerCard0`)) true)
  (`self.SetActorHiddenInGame` (`ChildActorComponent.ChildActor` (`self.DealerCard1`)) true)
  (`self.SetActorHiddenInGame` (`ChildActorComponent.ChildActor` (`self.DealerCard2`)) true)
  (set `self.NextPlayerCardIndex` 0)
  (set `self.NextDealerCardIndex` 0))

(fn `RevealDealerHandVisual`
  (bind _returnvalue (`self.GetDealerHand`))
  (bind (_deckstyle _suit _rank _fronttexture _backtexture) (break `BlackjackCardVisualData` (`BlackjackBlueprintLibrary.FindBlackjackCardVisualData` "/Game/Blackjack/Data/DT_BlackjackCardVisuals.DT_BlackjackCardVisuals" "CasinoRed" (`|GetArrayItem` _returnvalue))))
  (bind (_deckstyle_2 _suit_2 _rank_2 _fronttexture_2 _backtexture_2) (break `BlackjackCardVisualData` (`BlackjackBlueprintLibrary.FindBlackjackCardVisualData` "/Game/Blackjack/Data/DT_BlackjackCardVisuals.DT_BlackjackCardVisuals" "CasinoRed" (`|GetArrayItem` _returnvalue 1))))
  (bind (_deckstyle_3 _suit_3 _rank_3 _fronttexture_3 _backtexture_3) (break `BlackjackCardVisualData` (`BlackjackBlueprintLibrary.FindBlackjackCardVisualData` "/Game/Blackjack/Data/DT_BlackjackCardVisuals.DT_BlackjackCardVisuals" "CasinoRed" (`|GetArrayItem` _returnvalue 2))))
  (bind _asbp_blackjack_card (cast `/Game/Blackjack/BluePrint/Card/BP_BlackjackCard` (`ChildActorComponent.ChildActor` (`self.DealerCard0`))))
  (`/Game/Blackjack/BluePrint/Card/BP_BlackjackCard.InitializeCard` _asbp_blackjack_card _fronttexture _backtexture true)
  (bind _asbp_blackjack_card_2 (cast `/Game/Blackjack/BluePrint/Card/BP_BlackjackCard` (`ChildActorComponent.ChildActor` (`self.DealerCard1`))))
  (`/Game/Blackjack/BluePrint/Card/BP_BlackjackCard.InitializeCard` _asbp_blackjack_card_2 _fronttexture_2 _backtexture_2 true)
  (bind _asbp_blackjack_card_3 (cast `/Game/Blackjack/BluePrint/Card/BP_BlackjackCard` (`ChildActorComponent.ChildActor` (`self.DealerCard2`))))
  (`/Game/Blackjack/BluePrint/Card/BP_BlackjackCard.InitializeCard` _asbp_blackjack_card_3 _fronttexture_3 _backtexture_3 true))

(fn `UserConstructionScript`)