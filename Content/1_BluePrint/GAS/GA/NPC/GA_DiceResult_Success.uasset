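; Gameplay ability for a game NPC that plays its success montage when a dice result is won.
; On completion it clears the NPC's anim-play flag and, on the server, tells the overlapping first-person player's client to reopen dice betting before ending.
; Interruption or cancellation only clears the flag and ends the ability.
; An older direct OpenBetting call remains in the graph but never runs.
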(event `self.K2_ActivateAbility`
  (bind _asnpc_game (cast `NPC_Game` (`self.GetOwningActorFromActorInfo`)))
  (`AbilityTask_PlayMontageAndWait.CreatePlayMontageAndWaitProxy` "None" (`NPC_Game.GameSuccessMontage` _asnpc_game)
    (:`OnCompleted`
      (`NPC_Base.SetIsAnimPlay` _asnpc_game false)
      (`self.K2_HasAuthority`
        (:`True`
          (bind _returnvalue (`NPC_Base.GetOverlappingPlayer` _asnpc_game))
          (`/Engine/EditorBlueprintResources/StandardMacros.IsValid` _returnvalue
            (:`Is Valid`
              (bind _asbp_first_person_character (cast `/Game/1_BluePrint/Actor/BP_FirstPersonCharacter` _returnvalue)
                (:`then`
                  (`/Game/1_BluePrint/Actor/BP_FirstPersonCharacter.Client_ReopenDiceBetting` _asbp_first_person_character))
                (:`CastFailed`
                  _)))
            (:`Is Not Valid`
              _)))
        (:`False`
          _))
      (`self.K2_EndAbility`))
    (:`OnInterrupted`
      (`NPC_Base.SetIsAnimPlay` _asnpc_game false :!label _label)
      (`self.K2_EndAbility`))
    (:`OnCancelled`
      (goto _label))))