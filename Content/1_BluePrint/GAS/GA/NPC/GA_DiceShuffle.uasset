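; Gameplay ability that runs an NPC's dice shuffle when a player is overlapping the NPC.
; It plays the game start montage and waits for an animation gameplay event, then rolls a uniform random total and shows it on the dice game.
; After a delay, it compares the roll's parity to the NPC's selected value, activating the NPC Fail ability on a match or Success otherwise, then hides the dice and ends.
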(event `self.K2_ActivateAbility`
  (bind _asnpc_game (cast `NPC_Game` (`self.GetOwningActorFromActorInfo`)))
  (bind _output_get (set `self.GameNpc` _asnpc_game))
  (`/Engine/EditorBlueprintResources/StandardMacros.IsValid` (`NPC_Base.OverlappingPlayer` _asnpc_game)
    (:`Is Valid`
      (`AbilityTask_PlayMontageAndWait.CreatePlayMontageAndWaitProxy` "None" (`NPC_Game.GameStartMontage` _output_get) 1.0 "Default" true 1.0 0.0 true
        (:`then`
          (`AbilityTask_WaitGameplayEvent.WaitGameplayEvent` (struct :`TagName` "AnimEvent") null true
            (:`then`
              (`NPC_Base.SetIsAnimPlay` (`self.GameNpc`) true))
            (:`EventReceived`
              (bind _asbp_npc_dice (cast `/Game/1_BluePrint/NPC/BP_NPC_Dice` (`self.GetOwningActorFromActorInfo`)))
              (bind _output_get_2 (set `self.ResultValue` (`KismetMathLibrary.RandomIntegerInRange` 2 12)))
              (bind _returnvalue (`NPC_Dice.GetDiceGame` _asbp_npc_dice))
              (`DiceGame.SetDice` _returnvalue true _output_get_2)
              (`KismetSystemLibrary.Delay` 3.0)
              (if (== (mod _output_get_2 2) (`NPC_Dice.SelectedValue` _asbp_npc_dice))
                (bind _abilitysystemcomponent (`NPC_Base.AbilitySystemComponent` _asbp_npc_dice))
                (`AbilitySystemComponent.TryActivateAbilitiesByTag` _abilitysystemcomponent (`BlueprintGameplayTagLibrary.MakeLiteralGameplayTagContainer` (struct :`GameplayTags` (struct :`(TagName` "NPC.Fail")))) true)
                (else
                  (`AbilitySystemComponent.TryActivateAbilitiesByTag` _abilitysystemcomponent (`BlueprintGameplayTagLibrary.MakeLiteralGameplayTagContainer` (struct :`GameplayTags` (struct :`(TagName` "NPC.Success")))) true)))
              (`DiceGame.SetDice` _returnvalue false 0)
              (`self.K2_EndAbility`))))))
    (:`Is Not Valid`
      (`self.K2_EndAbility`))))