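; GA_Punch is a player Gameplay Ability that performs a punch on BP_FirstPersonCharacter.
; Both authority and client play the attack montage without root motion translation, ending the ability when it completes, blends out or is interrupted.
; Only the authority opens the character's PunchHitAvailable window on activation and closes it when the ability ends.
; Activation is blocked while any directional hit-reaction montage plays or no valid anim instance exists.
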(event `self.K2_OnEndAbility`
  (params (bWasCancelled :type Boolean))
  (bind _asbp_first_person_character (cast `/Game/1_BluePrint/Actor/BP_FirstPersonCharacter` (`self.GetAvatarActorFromActorInfo`)))
  (if (`Actor.HasAuthority` _asbp_first_person_character)
    (set `/Game/1_BluePrint/Actor/BP_FirstPersonCharacter.bPunchHitAvailable` false _asbp_first_person_character)))

(event `self.K2_ActivateAbility`
  (bind _asbp_first_person_character (cast `/Game/1_BluePrint/Actor/BP_FirstPersonCharacter` (`self.GetAvatarActorFromActorInfo`))
    (:`then`
      (if (`Actor.HasAuthority` _asbp_first_person_character)
        (set `/Game/1_BluePrint/Actor/BP_FirstPersonCharacter.bPunchHitAvailable` true _asbp_first_person_character)
        (`AbilityTask_PlayMontageAndWait.CreatePlayMontageAndWaitProxy` "None" "/Game/LJH/Animations/MM_Attack_02_Montage.MM_Attack_02_Montage" 1.0 "None" true 0.0
          (:`OnCompleted`
            _)
          (:`OnBlendOut`
            _)
          (:`OnInterrupted`
            _)
          (:`OnCancelled`
            _))
        (`self.K2_EndAbility`)
        (else
          (`AbilityTask_PlayMontageAndWait.CreatePlayMontageAndWaitProxy` "None" "/Game/LJH/Animations/MM_Attack_02_Montage.MM_Attack_02_Montage" 1.0 "None" true 0.0
            (:`OnCompleted`
              _)
            (:`OnBlendOut`
              _)
            (:`OnInterrupted`
              _)
            (:`OnCancelled`
              _))
          (`self.K2_EndAbility`))))
    (:`CastFailed`
      (`self.K2_EndAbility`))))

(fn `K2_CanActivateAbility`
  (params (ActorInfo :type "GameplayAbilityActorInfo Structure") (Handle :type "GameplayAbilitySpecHandle Structure"))
  (returns (RelevantTags :type "GameplayTagContainer Structure") (ReturnValue :type Boolean))
  (bind _returnvalue (`SkeletalMeshComponent.GetAnimInstance` (`.SkeletalMeshComponent` (break `GameplayAbilityActorInfo` ActorInfo))))
  (`/Engine/EditorBlueprintResources/StandardMacros.IsValid` _returnvalue
    (:`Is Valid`
      (return (struct) (not (or (`AnimInstance.Montage_IsActive` _returnvalue "/Game/LJH/Animations/MM_Hit_Back_02_Montage.MM_Hit_Back_02_Montage") (`AnimInstance.Montage_IsActive` _returnvalue "/Game/LJH/Animations/MM_Hit_Front_02_Montage.MM_Hit_Front_02_Montage") (`AnimInstance.Montage_IsActive` _returnvalue "/Game/LJH/Animations/MM_Hit_Left_02_Montage.MM_Hit_Left_02_Montage") (`AnimInstance.Montage_IsActive` _returnvalue "/Game/LJH/Animations/MM_Hit_Right_02_Montage.MM_Hit_Right_02_Montage")))))
    (:`Is Not Valid`
      (return (struct) false))))