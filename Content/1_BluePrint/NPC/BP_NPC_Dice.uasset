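; BP_NPC_Dice is an interactable NPC that opens betting for the player, likely for a dice game as its name suggests.
; On interact, it checks that the interacting character is locally controlled, casts it to BP_FirstPersonCharacter and calls OpenBetting on it.
; The betting logic itself lives outside this Blueprint, and its other events only forward to the parent class.
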(event `self.ReceiveBeginPlay`
  (`parent.ReceiveBeginPlay`))

(event `self.ReceiveActorBeginOverlap`
  (params (OtherActor :type "Actor Object Reference"))
  (`parent.ReceiveActorBeginOverlap` OtherActor))

(event `self.ReceiveTick`
  (params (DeltaSeconds :type "Float (single-precision)"))
  (`parent.ReceiveTick` DeltaSeconds))

(event `self.BP_OnInteract`
  (params (InteractingCharacter :type "casino_simulatorCharacter Object Reference"))
  (if (`self.IsLocallyControlled` InteractingCharacter)
    (bind _asbp_first_person_character (cast `/Game/1_BluePrint/Actor/BP_FirstPersonCharacter` InteractingCharacter))
    (`/Game/1_BluePrint/Actor/BP_FirstPersonCharacter.OpenBetting` _asbp_first_person_character)))

(fn `UserConstructionScript`
  (`parent.UserConstructionScript`))