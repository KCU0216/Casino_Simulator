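; BP_LadderMachine is an interactive machine actor that runs a ladder game on a widget-based screen.
; When the machine is ready, it extends the parent logic by binding itself to the screen and ladder widgets, turning the screen on and enabling input for the requesting player.
; Tab, Enter and the Left/Right arrows drive menu navigation, while any key resets the round if a result is open.
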(event `Key|Tab`
  (params (Key :type "Key Structure"))
  (:`Pressed`
    (`self.NavCycle`)))

(event `Key|Enter`
  (params (Key :type "Key Structure"))
  (:`Pressed`
    (`self.NavSelect`)))

(event `Key|Left`
  (params (Key :type "Key Structure"))
  (:`Pressed`
    (`self.NavLeft`)))

(event `Key|Right`
  (params (Key :type "Key Structure"))
  (:`Pressed`
    (`self.NavRight`)))

(event `Key|AnyKey`
  (params (Key :type "Key Structure"))
  (:`Pressed`
    (if (`self.bResultOpen`)
      (`self.ResetRound`))))

(event `self.OnMachineReady`
  (params (RequestingCharacter :type "casino_simulatorCharacter Object Reference"))
  (`parent.OnMachineReady` RequestingCharacter)
  (bind _aswbp_machine_screen (cast `/Game/KCU/Widget/WBP_MachineScreen` (`WidgetComponent.GetWidget` (`self.Widget`))))
  (set `/Game/KCU/Widget/WBP_MachineScreen.Machine` self _aswbp_machine_screen)
  (`LadderWidget.SetMachine` (`/Game/KCU/Widget/WBP_MachineScreen.WBP_LadderWidget` _aswbp_machine_screen) self)
  (`/Game/KCU/Widget/WBP_MachineScreen.TurnOnScreen` _aswbp_machine_screen)
  (bind _asplayer_controller (cast `PlayerController` (`Pawn.GetController` RequestingCharacter)))
  (`self.EnableInput` _asplayer_controller))

(fn `UserConstructionScript`)