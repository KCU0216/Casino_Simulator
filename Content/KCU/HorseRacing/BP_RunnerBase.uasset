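; Base runner Blueprint for the HorseRacing game that sets a racer's appearance from its stats.
; OnStatsUpdated walks a chain of Stats.Age thresholds, using Age as the selector for one of six character variants.
; Each band swaps the Skin skeletal mesh, its matching Anim Blueprint and the RunnerPortrait together.
; Ages above the last band leave the appearance unchanged, and no other event has logic.
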(event `self.OnStatsUpdated`
  (bind (_name _age) (break `RaceRunnerStats` (`self.Stats`)))
  (if (<= _age 64)
    (`SkeletalMeshComponent.SetSkeletalMeshAsset` (`self.Skin`) "/Game/KCU/MyContent/WarriorBunnyGirl/Mesh/SKM_WarriorBunnyGirl_LINGERIE.SKM_WarriorBunnyGirl_LINGERIE")
    (`SkeletalMeshComponent.SetAnimInstanceClass` (`self.Skin`) "/Game/KCU/HorseRacing/ABP_RunnerBunny.ABP_RunnerBunny_C")
    (set `self.RunnerPortrait` "/Game/KCU/HorseRacing/runner_bunny_woman.runner_bunny_woman")
    (elif (<= _age 74)
      (`SkeletalMeshComponent.SetSkeletalMeshAsset` (`self.Skin`) "/Game/KCU/HorseRacing/rig-animated-fbx/blind_man_ani.blind_man_ani")
      (`SkeletalMeshComponent.SetAnimInstanceClass` (`self.Skin`) "/Game/KCU/HorseRacing/rig-animated-fbx/ABP_Blind.ABP_Blind_C")
      (set `self.RunnerPortrait` "/Game/KCU/HorseRacing/runner_blind_man.runner_blind_man")
      (elif (<= _age 84)
        (`SkeletalMeshComponent.SetSkeletalMeshAsset` (`self.Skin`) "/Game/KCU/HorseRacing/rig-animated-fbx/cane_man_ani.cane_man_ani")
        (`SkeletalMeshComponent.SetAnimInstanceClass` (`self.Skin`) "/Game/KCU/HorseRacing/rig-animated-fbx/ABP_Cane.ABP_Cane_C")
        (set `self.RunnerPortrait` "/Game/KCU/HorseRacing/runner_cane_man.runner_cane_man")
        (elif (<= _age 94)
          (`SkeletalMeshComponent.SetSkeletalMeshAsset` (`self.Skin`) "/Game/KCU/HorseRacing/rig-animated-fbx/wheelchair_man_ani.wheelchair_man_ani")
          (`SkeletalMeshComponent.SetAnimInstanceClass` (`self.Skin`) "/Game/KCU/HorseRacing/rig-animated-fbx/ABP_Wheel.ABP_Wheel_C")
          (set `self.RunnerPortrait` "/Game/KCU/HorseRacing/runner_wheelchair_man.runner_wheelchair_man")
          (elif (<= _age 104)
            (`SkeletalMeshComponent.SetSkeletalMeshAsset` (`self.Skin`) "/Game/KCU/HorseRacing/rig-animated-fbx/blind_woman_ani.blind_woman_ani")
            (`SkeletalMeshComponent.SetAnimInstanceClass` (`self.Skin`) "/Game/KCU/HorseRacing/rig-animated-fbx/ABP_BlindW.ABP_BlindW_C")
            (set `self.RunnerPortrait` "/Game/KCU/HorseRacing/runner_blind_woman.runner_blind_woman")
            (elif (<= _age 114)
              (`SkeletalMeshComponent.SetSkeletalMeshAsset` (`self.Skin`) "/Game/LJH/Bunny/Dolbani_v2/Meshes/SK_Dolbani_v2.SK_Dolbani_v2")
              (`SkeletalMeshComponent.SetAnimInstanceClass` (`self.Skin`) "/Game/LJH/Bunny/Dolbani_v2/Meshes/ABP_Runner_Dolbani.ABP_Runner_Dolbani_C")
              (set `self.RunnerPortrait` "/Game/KCU/HorseRacing/runner_bunny_mascot.runner_bunny_mascot"))))))))

(fn `UserConstructionScript`)