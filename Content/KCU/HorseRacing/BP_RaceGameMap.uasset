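; BP_RaceGameMap drives a scene-capture broadcast camera for the horse race, apparently for a billboard.
; When the billboard phase changes to Racing, a looping timer captures RaceCapture at about 30 fps; other phases stop the timer.
; During Racing, Tick eases the capture toward a raised point offset along the leading runner's forward vector, changing only its location, not its rotation.
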(event `self.ReceiveBeginPlay`)

(event `self.OnBillboardPhaseChanged`
  (params (NewPhase :type "ERacePhase Enum" :default "Idle"))
  (`KismetSystemLibrary.K2_ClearAndInvalidateTimerHandle` (`self.CaptureTimerHandle`))
  (if (`|EnumEquality` NewPhase "Racing")
    (bind _returnvalue (`KismetSystemLibrary.K2_SetTimerDelegate` (delegate `CaptureRaceFrame`) 0.0333 true true))
    (set `self.CaptureTimerHandle` _returnvalue)))

(event `CaptureRaceFrame`
  (`SceneCaptureComponent2D.CaptureScene` (`self.RaceCapture`)))

(event `self.ReceiveTick`
  (params (DeltaSeconds :type "Float (single-precision)"))
  (bind _broadcasttarget (`self.BroadcastTarget`))
  (if (`|EnumEquality` (`self.Phase`) "Racing")
    (bind _output_get (set `self.BroadcastTarget` (`self.GetLeadingRunner`)))
    (if (`KismetSystemLibrary.IsValid` _output_get)
      (`SceneComponent.K2_SetWorldLocation` (`self.RaceCapture`) (`KismetMathLibrary.VInterpTo` (`SceneComponent.K2_GetComponentLocation` (`self.RaceCapture`)) (+ (+ (`self.K2_GetActorLocation` _broadcasttarget) (* (`self.GetActorForwardVector` _broadcasttarget) (`self.CameraDistance`))) (`KismetMathLibrary.MakeVector` 0.0 0.0 (`self.CameraHeight`))) DeltaSeconds (`self.FollowSpeed`)) false false))))

(fn `UserConstructionScript`)