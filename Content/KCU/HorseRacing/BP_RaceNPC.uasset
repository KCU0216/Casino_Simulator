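; BP_RaceNPC is an interactable NPC for the horse racing game that loops an idle animation.
; On interaction, it creates a WBP_RaceNPCWidget, passing in the interacting first-person character and the RaceManager taken from its owner.
; The casino player controller then blends the camera to the NPC's interaction target and shows the widget in interaction UI mode.
; Interaction silently does nothing unless the NPC's owner is a RaceManager.
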(event `self.ReceiveBeginPlay`
  (`SkeletalMeshComponent.PlayAnimation` (`self.Mesh`) "/Game/KCU/MyContent/WarriorBunnyGirl/Demo/AS_ThirdPersonIdle.AS_ThirdPersonIdle" true))

(event `self.BP_OnInteract`
  (params (InteractingCharacter :type "casino_simulatorCharacter Object Reference"))
  (bind _asrace_manager (cast `RaceManager` (`self.GetOwner`)))
  (bind _asbp_first_person_character (cast `/Game/1_BluePrint/Actor/BP_FirstPersonCharacter` InteractingCharacter))
  (bind _ascasino_simulator_player_controller (cast `casino_simulatorPlayerController` (`self.GetController` InteractingCharacter)))
  (bind _returnvalue (`|CreateWidget` "/Game/KCU/HorseRacing/WBP_RaceNPCWidget.WBP_RaceNPCWidget_C" _ascasino_simulator_player_controller _asrace_manager _asbp_first_person_character))
  (`casino_simulatorPlayerController.EnterInteractionUIMode` _ascasino_simulator_player_controller (`self.GetInteractionCameraTarget`) 0.35)
  (`casino_simulatorPlayerController.ShowInteractionUI` _ascasino_simulator_player_controller _returnvalue)
  (`KismetSystemLibrary.PrintString` (`KismetStringLibrary.Conv_BoolToString` (`casino_simulatorPlayerController.bInteractionUIOpen` _ascasino_simulator_player_controller))))

(fn `UserConstructionScript`)