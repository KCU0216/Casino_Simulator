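; BP_MineNPC is an interactable mine shop NPC that sells Power and Speed upgrades to the player and plays a looping idle animation.
; Interacting creates WBP_MineUpgradeWidget and has the player controller blend the camera into interaction UI mode.
; Widget button events send purchase requests to MiningShopComponent, whose success and failure events feed results back to the widget.
; The exit button closes the interaction and removes the widget.
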(event `self.BP_OnInteract`
  (params (InteractingCharacter :type "casino_simulatorCharacter Object Reference"))
  (bind _asbp_first_person_character (cast `/Game/1_BluePrint/Actor/BP_FirstPersonCharacter` InteractingCharacter))
  (set `self.Player` _asbp_first_person_character)
  (bind _returnvalue (`|CreateWidget` "/Game/KCU/Mine/WBP_MineUpgradeWidget.WBP_MineUpgradeWidget_C"))
  ; 버튼 바인딩
  (bind _output_get (set `self.MineWidget` _returnvalue))
  (add `/Game/KCU/Mine/WBP_MineUpgradeWidget.파워업버튼눌렸다잉` _output_get (delegate `파워업버튼눌렸다잉_Event`))
  (add `/Game/KCU/Mine/WBP_MineUpgradeWidget.스피드업버튼눌렸따잉` (`self.MineWidget`) (delegate `스피드업버튼눌렸따잉_Event`))
  (add `/Game/KCU/Mine/WBP_MineUpgradeWidget.나가기눌렀다잉` (`self.MineWidget`) (delegate `나가기버튼눌렀다잉_Event`))
  ; 구매 성공/실패시 텍스트 바인딩
  (add `MiningShopComponent.OnPurchaseCompleted` (`self.MiningShopComponent`) (delegate `구매성공시이벤트`))
  (add `MiningShopComponent.OnPurchaseFailed` (`self.MiningShopComponent`) (delegate `구매실패시이벤트`))
  (`UserWidget.AddToViewport` (`self.MineWidget`) 0)
  (bind _ascasino_simulator_player_controller (cast `casino_simulatorPlayerController` (`self.GetController` InteractingCharacter)))
  (`casino_simulatorPlayerController.EnterInteractionUIMode` _ascasino_simulator_player_controller (`self.GetInteractionCameraTarget`) 0.35))

(event `구매성공시이벤트`
  (params (UpgradeType :type "EMiningShopUpgradeType Enum" :default "Power") (TotalPrice :type Integer))
  ; 구매 성공/실패시 텍스트 바인딩
  (`/Game/KCU/Mine/WBP_MineUpgradeWidget.ShowPurchaseCompleted` (`self.MineWidget`) UpgradeType TotalPrice))

(event `구매실패시이벤트`
  (params (UpgradeType :type "EMiningShopUpgradeType Enum" :default "Power") (Reason :type String))
  ; 구매 성공/실패시 텍스트 바인딩
  (`/Game/KCU/Mine/WBP_MineUpgradeWidget.ShowPurchaseFailed` (`self.MineWidget`) UpgradeType Reason))

(event `파워업버튼눌렸다잉_Event`
  (`MiningShopComponent.RequestBuyUpgrade` (`self.MiningShopComponent`) (`self.Player`) "Power"))

(event `스피드업버튼눌렸따잉_Event`
  (`MiningShopComponent.RequestBuyUpgrade` (`self.MiningShopComponent`) (`self.Player`) "Speed"))

(event `나가기버튼눌렀다잉_Event`
  (bind _ascasino_simulator_player_controller (cast `casino_simulatorPlayerController` (`self.GetController` (`self.Player`))))
  (`casino_simulatorPlayerController.CloseCurrentInteraction` _ascasino_simulator_player_controller)
  (`Widget.RemoveFromParent` (`self.MineWidget`)))

(event `self.ReceiveBeginPlay`
  (`SkeletalMeshComponent.PlayAnimation` (`self.Mesh`) "/Game/KCU/MyContent/WarriorBunnyGirl/Demo/AS_ThirdPersonIdle.AS_ThirdPersonIdle" true))

(fn `UserConstructionScript`)