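; Blackjack card actor that shows front and back textures, flips face up or down, and animates being dealt to a target.
; InitializeCard, SetFaceUp and the texture and face RepNotifies feed ApplyCardVisuals, which creates dynamic materials and rotates the visual root.
; DealTo scales timeline play rate to the requested duration, driving a sine-arc move with optional rotation blend and a landing sound.
; AttachToDealerHand snaps the card to the dealer's hand socket.
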(event `self.ReceiveBeginPlay`
  (`self.ApplyCardVisuals`))

(fn `ApplyCardVisuals`
  (bind _returnvalue (`PrimitiveComponent.CreateDynamicMaterialInstance` (`self.FrontFace`) 0 "/Game/Blackjack/BluePrint/Card/Material/M_CardFace.M_CardFace" "None"))
  (bind _output_get (set `self.FrontMID` _returnvalue))
  (`MaterialInstanceDynamic.SetTextureParameterValue` _output_get "CardTexture" (`self.FrontTexture`))
  (bind _returnvalue_2 (`PrimitiveComponent.CreateDynamicMaterialInstance` (`self.BackFace`) 0 "/Game/Blackjack/BluePrint/Card/Material/M_CardBack.M_CardBack" "None"))
  (bind _output_get_2 (set `self.BackMID` _returnvalue_2))
  (`MaterialInstanceDynamic.SetTextureParameterValue` _output_get_2 "BackTexture" (`self.BackTexture`))
  (if (`self.bFaceUp`)
    (`SceneComponent.K2_SetRelativeRotation` :`self` (`self.CardVisualRoot`))
    (else
      (`SceneComponent.K2_SetRelativeRotation` (`self.CardVisualRoot`) (struct :`Pitch` 180.0) false false))))

(fn `AttachToDealerHand`
  (params (DealerMesh :type "SkeletalMeshComponent Object Reference"))
  (`self.K2_AttachToComponent` DealerMesh "Socket_CardDeal_R" "SnapToTarget" "SnapToTarget" "KeepWorld"))

(fn `DealTo`
  (params (TargetTransform :type "Transform Structure") (Duration :type "Float (double-precision)") (isRot :type Boolean))
  (bind _tl_deal (`self.TL_Deal`))
  (set `self.DealStartTransform` (`self.GetTransform`))
  (set `self.Is Rot` isRot)
  (set `self.DealTargetTransform` (`KismetMathLibrary.MakeTransform` (.location TargetTransform) (.rotation TargetTransform) (.scale TargetTransform)))
  (set `self.DealDuration` Duration)
  (`TimelineComponent.SetPlayRate` _tl_deal (/ (`TimelineComponent.GetTimelineLength` _tl_deal) (`KismetMathLibrary.FMax` Duration 0.01)))
  (`TimelineComponent.PlayFromStart` _tl_deal))

(fn `InitializeCard`
  (params (InFrontTexture :type "Texture2D Object Reference") (InBackTexture :type "Texture2D Object Reference") (InFaceUp :type Boolean))
  (set `self.FrontTexture` (select `bool` InFaceUp :`true` InFrontTexture))
  (set `self.BackTexture` InBackTexture)
  (set `self.bFaceUp` InFaceUp)
  (`self.ApplyCardVisuals`))

(fn `OnRep_BackTexture`
  (`self.ApplyCardVisuals`))

(fn `OnRep_bFaceUp`
  (`self.ApplyCardVisuals`))

(fn `OnRep_FrontTexture`
  (`self.ApplyCardVisuals`))

(fn `SetFaceUp`
  (params (InFaceUp :type Boolean))
  (set `self.bFaceUp` InFaceUp)
  (`self.ApplyCardVisuals`))

(fn `UserConstructionScript`)