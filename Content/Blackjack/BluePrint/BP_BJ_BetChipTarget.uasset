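; BP_BJ_BetChipTarget is a blackjack bet chip target that opens the betting keypad when a character interacts with it.
; OnLocalBlackjackInteract lazily creates WBP_BlackjackHUD for the interacting character's PlayerController, adds it to the viewport and caches the reference.
; Each interaction, whether creating or reusing that HUD, calls InitializeBlackjackHUD and then OpenBetKeypad.
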(event `self.BP_OnLocalBlackjackInteract`
  (params (InteractingCharacter :type "casino_simulatorCharacter Object Reference") (Table :type "BlackjackTableActor Object Reference") (Action :type "EBlackjackTableInteractionAction Enum" :default "OpenBetting"))
  (bind _blackjackhudref (`self.BlackjackHUDRef`))
  (`/Engine/EditorBlueprintResources/StandardMacros.IsValid` _blackjackhudref
    (:`Is Valid`
      (`/Game/Blackjack/BluePrint/Widget/WBP_BlackjackHUD.InitializeBlackjackHUD` _blackjackhudref)
      (`/Game/Blackjack/BluePrint/Widget/WBP_BlackjackHUD.OpenBetKeypad` _blackjackhudref))
    (:`Is Not Valid`
      (bind `_as플레이어_컨트롤러` (cast `PlayerController` (`Pawn.GetController` InteractingCharacter)))
      (bind _returnvalue (`|CreateWidget` "/Game/Blackjack/BluePrint/Widget/WBP_BlackjackHUD.WBP_BlackjackHUD_C" `_as플레이어_컨트롤러` InteractingCharacter))
      (set `self.BlackjackHUDRef` _returnvalue)
      (`UserWidget.AddToViewport` _blackjackhudref 0)
      (`/Game/Blackjack/BluePrint/Widget/WBP_BlackjackHUD.InitializeBlackjackHUD` _blackjackhudref)
      (`/Game/Blackjack/BluePrint/Widget/WBP_BlackjackHUD.OpenBetKeypad` _blackjackhudref))))

(fn `UserConstructionScript`)