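; Blackjack table actor that turns round events into card visuals for four seats and the dealer.
; Deal events spawn data-table-textured cards at the deck, presented by the child-actor dealer or moved directly without one.
; A seat/hand/card string-keyed map lets splits re-key and slide cards, while hole-card reveal re-initializes the dealer's second card face up.
; Round completion releases leaving seats, clears cards and, after delays, resets and reopens betting.
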(event `self.ReceiveBeginPlay`
  (bind _asbp_npc_blackjack_dealer (cast `/Game/Blackjack/BluePrint/BP_NPC_BlackjackDealer` (`ChildActorComponent.ChildActor` (`self.BP_NPC_BlackjackDealer`))))
  (set `self.DealerActor` _asbp_npc_blackjack_dealer)
  (set `/Game/Blackjack/BluePrint/BP_NPC_BlackjackDealer.BlackjackTable` self _asbp_npc_blackjack_dealer)
  (add `self.OnPlayerHandCardDealt` (delegate `HandlePlayerHandCardDealt`))
  (add `self.OnDealerCardDealt` (delegate `HandleDealerCardDealt`))
  (add `self.OnDealerHoleCardRevealed` (delegate `HandleDealerHoleCardRevealed`))
  (add `self.OnPlayerHandsSplit` (delegate `HandlePlayerHandsSplit`))
  (add `self.OnRoundCompleted` (delegate `HandleRoundCompleted`))
  (add `self.OnTableChanged` (delegate `HandleTableChanged`))
  (add `self.OnDealerTableVisualReset` (delegate `HandleDealerTableVisualReset`))
  (`self.ResetVisualCardCounts`))

(event `HandleDealerHoleCardRevealed` :!signature `self.OnDealerHoleCardRevealed`
  (params (SeatIndex :type Integer) (Card :type "BlackjackCard Structure (by ref)"))
  (`self.RevealDealerHoleCardVisual` Card))

(event `HandleDealerCardDealt` :!signature `self.OnDealerCardDealt`
  (params (SeatIndex :type Integer) (Card :type "BlackjackCard Structure (by ref)"))
  (`self.DealVisualCardToDealer` Card))

(event `HandleTableChanged`
  (switch `EBlackjackRoundState` (`self.GetRoundState`)))

(event `HandlePlayerHandCardDealt` :!signature `self.OnPlayerHandCardDealt`
  (params (SeatIndex :type Integer) (HandIndex :type Integer) (CardIndex :type Integer) (Card :type "BlackjackCard Structure (by ref)"))
  (`self.DealVisualCardToPlayer` SeatIndex Card HandIndex CardIndex))

(event `HandlePlayerHandsSplit` :!signature `self.OnPlayerHandsSplit`
  (params (SeatIndex :type Integer) (SeatState :type "BlackjackSeatState Structure (by ref)"))
  (`self.ApplySplitCardVisuals` SeatIndex SeatState))

(event `HandleDealerTableVisualReset`
  (`self.ClearBlackjackCardVisuals`))

(event `HandleRoundCompleted`
  (`KismetSystemLibrary.Delay` 3.0)
  (`self.ReleaseSeatsLeavingAfterRound`)
  (`self.ClearBlackjackCardVisuals`)
  (`KismetSystemLibrary.Delay` 3.0)
  (`self.ResetRound`)
  (`self.StartBettingWindow` 10.0))

(fn `ApplySplitCardVisuals`
  (params (SeatIndex :type Integer) (SeatState :type "BlackjackSeatState Structure"))
  (bind (_seatindex _occupant _hands) (break `BlackjackSeatState` SeatState))
  (bind _playercardvisualmap (`self.PlayerCardVisualMap`))
  (bind _cards (break `BlackjackHand` (`|GetArrayItem` _hands)))
  (bind _cards_2 (break `BlackjackHand` (`|GetArrayItem` _hands 1)))
  (if (`KismetArrayLibrary.Array_IsValidIndex` _hands 1)
    (bind _key (`self.MakePlayerCardKey` SeatIndex 0 1))
    (bind (_value _returnvalue) (`BlueprintMapLibrary.Map_Find` _playercardvisualmap _key))
    (if _returnvalue
      (`/Engine/EditorBlueprintResources/StandardMacros.IsValid` _value
        (:`Is Valid`
          (set `self.MovedCard` _value)
          (`BlueprintMapLibrary.Map_Remove` _playercardvisualmap _key)
          (bind _key_2 (`self.MakePlayerCardKey` SeatIndex 1))
          (`BlueprintMapLibrary.Map_Add` _playercardvisualmap _key_2 (`self.MovedCard`))
          (`self.MovePlayerCardVisual` SeatIndex)
          (`self.MovePlayerCardVisual` SeatIndex 1)
          (if (and (`KismetArrayLibrary.Array_IsValidIndex` _cards 1) (`KismetArrayLibrary.Array_IsValidIndex` _cards_2 1))
            (`self.DealVisualCardToPlayer` SeatIndex (`|GetArrayItem` _cards 1) 0 1)
            (`self.DealVisualCardToPlayer` SeatIndex (`|GetArrayItem` _cards_2 1) 1 1)))))))

(fn `ClearBlackjackCardVisuals`
  (bind _allvisualcards (`self.AllVisualCards`))
  (bind _playervisualcardcounts (`self.PlayerVisualCardCounts`))
  (for _array_element _allvisualcards
    (`/Engine/EditorBlueprintResources/StandardMacros.IsValid` _array_element
      (:`Is Valid`
        (`self.K2_DestroyActor` _array_element))))
  (`KismetArrayLibrary.Array_Clear` _allvisualcards)
  (`KismetArrayLibrary.Array_Clear` (`self.DealerVisualCards`))
  (set `self.DealerCardCount` 0)
  (`BlueprintMapLibrary.Map_Clear` (`self.PlayerCardVisualMap`))
  (`KismetArrayLibrary.Array_Clear` _playervisualcardcounts)
  (`KismetArrayLibrary.Array_Add` _playervisualcardcounts)
  (`KismetArrayLibrary.Array_Add` _playervisualcardcounts)
  (`KismetArrayLibrary.Array_Add` _playervisualcardcounts)
  (`KismetArrayLibrary.Array_Add` _playervisualcardcounts))

(fn `ClearTableVisualCards`)

(fn `DealVisualCardToDealer`
  (params (Card :type "BlackjackCard Structure"))
  (bind _dealercardcount (`self.DealerCardCount`))
  (bind _dealeractor (`self.DealerActor`))
  (bind _targettransform (`self.GetDealerCardTargetTransform` _dealercardcount))
  (bind _spawnedcard (`self.SpawnAndInitializeCardVisual` Card (`SceneComponent.K2_GetComponentToWorld` (`self.DeckVisualPoint`))))
  (`KismetArrayLibrary.Array_Add` (`self.DealerVisualCards`) _spawnedcard)
  (`KismetArrayLibrary.Array_Add` (`self.AllVisualCards`) _spawnedcard)
  (if (`KismetSystemLibrary.IsValid` _dealeractor)
    (`BlackjackDealerVisual.PresentCard` _dealeractor _spawnedcard _targettransform 0.25 -1)
    (else
      (`/Game/Blackjack/BluePrint/Card/BP_BlackjackCard.DealTo` _spawnedcard _targettransform 0.25 false)))
  (set `self.DealerCardCount` (+ _dealercardcount 1)))

(fn `DealVisualCardToPlayer`
  (params (SeatIndex :type Integer) (Card :type "BlackjackCard Structure") (HandIndex :type Integer) (CardIndex :type Integer))
  (bind _dealeractor (`self.DealerActor`))
  (bind (_targettransform _bvalid) (`self.GetPlayerHandCardTargetTransform` SeatIndex HandIndex CardIndex))
  (if _bvalid
    (bind _spawnedcard (`self.SpawnAndInitializeCardVisual` Card (`SceneComponent.K2_GetComponentToWorld` (`self.DeckVisualPoint`))))
    (`/Engine/EditorBlueprintResources/StandardMacros.IsValid` _spawnedcard
      (:`Is Valid`
        (`KismetArrayLibrary.Array_Add` (`self.AllVisualCards`) _spawnedcard)
        (bind _key (`self.MakePlayerCardKey` SeatIndex HandIndex CardIndex))
        (`BlueprintMapLibrary.Map_Add` (`self.PlayerCardVisualMap`) _key _spawnedcard)
        (if (`KismetSystemLibrary.IsValid` _dealeractor)
          (`BlackjackDealerVisual.PresentCard` _dealeractor _spawnedcard _targettransform 0.25 SeatIndex)
          (else
            (`/Game/Blackjack/BluePrint/Card/BP_BlackjackCard.DealTo` _spawnedcard _targettransform 0.25 true)))))))

(fn `GetDealerCardTargetTransform`
  (params (CardIndex :type Integer))
  (returns (TargetTransform :type "Transform Structure"))
  (bind _rotation (.rotation (`SceneComponent.K2_GetComponentToWorld` (`self.DealerCardRoot`))))
  (return (`KismetMathLibrary.MakeTransform` (+ (* (* (`KismetMathLibrary.Conv_IntToDouble` CardIndex) 8.0) (`KismetMathLibrary.GetForwardVector` _rotation)) (.location (`SceneComponent.K2_GetComponentToWorld` (`self.DealerCardRoot`)))) (`KismetMathLibrary.ComposeRotators` _rotation (`KismetMathLibrary.MakeRotator` 0.0)) (.scale (`SceneComponent.K2_GetComponentToWorld` (`self.DealerCardRoot`))))))

(fn `GetPlayerCardTargetTransform`
  (params (SeatIndex :type Integer) (CardIndex :type Integer))
  (returns (TargetTransform :type "Transform Structure") (bValid :type Boolean))
  (bind _rotation (.rotation (`SceneComponent.K2_GetComponentToWorld` (`self.BaseCardPoint`))))
  (switch `int` SeatIndex
    (:`Default`
      (set `self.OutValid` false))
    (:`0`
      (set `self.BaseCardPoint` (`self.Player0CardPoint_0`))
      (set `self.OutTargetTransform` (`KismetMathLibrary.MakeTransform` (+ (.location (`SceneComponent.K2_GetComponentToWorld` (`self.BaseCardPoint`))) (* (`KismetMathLibrary.GetForwardVector` _rotation) (* (`KismetMathLibrary.Conv_IntToDouble` CardIndex) 8.0))) (`KismetMathLibrary.ComposeRotators` _rotation (`KismetMathLibrary.MakeRotator` 0.0)) (.scale (`SceneComponent.K2_GetComponentToWorld` (`self.BaseCardPoint`)))) :!label _label)
      (set `self.OutValid` true))
    (:`1`
      (set `self.BaseCardPoint` (`self.Player1CardPoint_1`))
      (goto _label))
    (:`2`
      (set `self.BaseCardPoint` (`self.Player2CardPoint_2`))
      (goto _label))
    (:`3`
      (set `self.BaseCardPoint` (`self.Player3CardPoint_3`))
      (goto _label)))
  (return (`self.OutTargetTransform`) (`self.OutValid`)))

(fn `GetPlayerHandCardTargetTransform`
  (params (SeatIndex :type Integer) (HandIndex :type Integer) (CardIndex :type Integer))
  (returns (TargetTransform :type "Transform Structure") (bValid :type Boolean))
  (bind (_targettransform _bvalid) (`self.GetPlayerCardTargetTransform` SeatIndex CardIndex))
  (bind _rotation (.rotation _targettransform))
  (return (`KismetMathLibrary.MakeTransform` (+ (.location _targettransform) (* (`KismetMathLibrary.GetForwardVector` _rotation) (* HandIndex 25))) _rotation (.scale _targettransform)) _bvalid))

(fn `MakePlayerCardKey`
  (params (SeatIndex :type Integer) (HandIndex :type Integer) (CardIndex :type Integer))
  (returns (Key :type String))
  (return (`KismetTextLibrary.Conv_TextToString` (`|FormatText` "{Seat}_{Hand}_{Card}" SeatIndex HandIndex CardIndex))))

(fn `MovePlayerCardVisual`
  (params (SeatIndex :type Integer) (HandIndex :type Integer) (CardIndex :type Integer))
  (bind _key (`self.MakePlayerCardKey` SeatIndex HandIndex CardIndex))
  (bind (_value _returnvalue) (`BlueprintMapLibrary.Map_Find` (`self.PlayerCardVisualMap`) _key))
  (if _returnvalue
    (`/Engine/EditorBlueprintResources/StandardMacros.IsValid` _value
      (:`Is Valid`
        (bind (_targettransform _bvalid) (`self.GetPlayerHandCardTargetTransform` SeatIndex HandIndex CardIndex))
        (if _bvalid
          (`/Game/Blackjack/BluePrint/Card/BP_BlackjackCard.DealTo` _value _targettransform 0.3 true))))))

(fn `ReleaseCurrentCardToPoint`
  (bind _currentdealingcard (`self.CurrentDealingCard`))
  (`/Engine/EditorBlueprintResources/StandardMacros.IsValid` _currentdealingcard
    (:`Is Valid`
      (`self.K2_DetachFromActor` _currentdealingcard "KeepWorld" "KeepWorld" "KeepWorld")
      (`/Game/Blackjack/BluePrint/Card/BP_BlackjackCard.DealTo` _currentdealingcard (`SceneComponent.K2_GetComponentToWorld` (`self.Player0CardPoint_0`)) 0.25 false))))

(fn `ResetVisualCardCounts`
  (set `self.PlayerCardCounts` (`|MakeArray` 0 0 0 0))
  (set `self.DealerCardCount` 0))

(fn `RevealDealerHoleCardVisual`
  (params (Card :type "BlackjackCard Structure"))
  (bind (_outvisualdata _returnvalue) (`BlackjackBlueprintLibrary.FindBlackjackCardVisualData` "/Game/Blackjack/Data/DT_BlackjackCardVisuals.DT_BlackjackCardVisuals" "CasinoRed" Card))
  (bind (_deckstyle _suit _rank _fronttexture _backtexture) (break `BlackjackCardVisualData` _outvisualdata))
  (bind _output (`|GetArrayItem` (`self.DealerVisualCards`) 1))
  (`/Engine/EditorBlueprintResources/StandardMacros.IsValid` _output
    (:`Is Valid`
      (if _returnvalue
        (`/Game/Blackjack/BluePrint/Card/BP_BlackjackCard.InitializeCard` _output _fronttexture _backtexture true)))))

(fn `SpawnAndInitializeCardVisual`
  (params (Card :type "BlackjackCard Structure") (StartTransform :type "Transform Structure"))
  (returns (SpawnedCard :type "/Game/Blackjack/BluePrint/Card/BP_BlackjackCard Object Reference"))
  (bind (_deckstyle _suit _rank _fronttexture _backtexture) (break `BlackjackCardVisualData` (`BlackjackBlueprintLibrary.FindBlackjackCardVisualData` "/Game/Blackjack/Data/DT_BlackjackCardVisuals.DT_BlackjackCardVisuals" "CasinoRed" Card)))
  (bind _returnvalue (`|SpawnActorFromClass` "/Game/Blackjack/BluePrint/Card/BP_BlackjackCard.BP_BlackjackCard_C" StartTransform "AlwaysSpawn" "MultiplyWithRoot" null null))
  (`/Game/Blackjack/BluePrint/Card/BP_BlackjackCard.InitializeCard` _returnvalue _fronttexture _backtexture (`.bFaceUp` (break `BlackjackCard` Card)))
  (return _returnvalue))

(fn `Test_Bet100`
  (bind _ascasino_simulator_character (cast `casino_simulatorCharacter` (`GameplayStatics.GetPlayerCharacter` 0)))
  (`BlackjackPlayerComponent.PlaceBet` (`casino_simulatorCharacter.GetBlackjackPlayerComponent` _ascasino_simulator_character) 100))

(fn `Test_Hit`
  (bind _ascasino_simulator_character (cast `casino_simulatorCharacter` (`GameplayStatics.GetPlayerCharacter` 0)))
  (`BlackjackPlayerComponent.Hit` (`casino_simulatorCharacter.GetBlackjackPlayerComponent` _ascasino_simulator_character)))

(fn `Test_Stand`
  (bind _ascasino_simulator_character (cast `casino_simulatorCharacter` (`GameplayStatics.GetPlayerCharacter` 0)))
  (`BlackjackPlayerComponent.Stand` (`casino_simulatorCharacter.GetBlackjackPlayerComponent` _ascasino_simulator_character)))

(fn `Test_StartRound`
  (`self.ResetVisualCardCounts`)
  (bind _ascasino_simulator_character (cast `casino_simulatorCharacter` (`GameplayStatics.GetPlayerCharacter` 0)))
  (bind _returnvalue (`BlackjackPlayerComponent.StartRound` (`casino_simulatorCharacter.GetBlackjackPlayerComponent` _ascasino_simulator_character)))
  (if _returnvalue
    (`KismetSystemLibrary.PrintString` "ㅐ")
    (else
      (`KismetSystemLibrary.PrintString` "ㅌ"))))

(fn `TestDealOneCard`
  (bind _dealeractor (`self.DealerActor`))
  (bind _returnvalue (`|SpawnActorFromClass` (`self.CardClass`) (`SceneComponent.K2_GetComponentToWorld` (`self.DeckVisualPoint`)) "Undefined" "MultiplyWithRoot" null null))
  (set `self.CurrentDealingCard` _returnvalue)
  (`/Game/Blackjack/BluePrint/Card/BP_BlackjackCard.InitializeCard` _returnvalue (`self.TestFrontTexture`) (`self.TestBackTexture`) false)
  (`/Game/Blackjack/BluePrint/Card/BP_BlackjackCard.AttachToDealerHand` (`self.CurrentDealingCard`) (`BlackjackDealerVisual.Mesh` _dealeractor))
  (`BlackjackDealerVisual.PlayAnimMontage` _dealeractor "/Game/Blackjack/BluePrint/Animation/Dealer/Retargeted/AS_Dealer_BJ_Card_Deal_P4_Montage_WBG.AS_Dealer_BJ_Card_Deal_P4_Montage_WBG" 1.0 "None"))

(fn `UserConstructionScript`)